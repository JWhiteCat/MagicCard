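; Game mode for a two-player tower-and-resource card game that holds both players' state and decides when a match ends.
; BeginPlay shows the mouse cursor and opens the main menu, while Tick polls VictoryConditions unless IsTest is set.
; A round limit gives a draw, while tower height, tower destruction or running out of cards decides a winner.
; Each ending resets all match variables, clears widgets and shows a game-over widget with the result.
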(event EventBeginPlay
  (Utilities|FlowControl|Sequence
    (:then_0
      (Variables|/Script/Engine.PlayerController|SetbShowMouseCursor (Game|GetPlayerController 0) true)
      (bind _returnvalue (UserInterface|CreateWidget "/Game/BluePrints/MainMenu.MainMenu_C"))
      (UserInterface|Viewport|AddtoViewport _returnvalue 0))))

(event EventTick
  (params (DeltaSeconds :type Float%20%28single-precision%29))
  (if (not (Variables|Default|GetIsTest))
    (CallFunction|VictoryConditions)))

(fn ConstructionScript)

(fn VictoryConditions
  (Utilities|FlowControl|Sequence
    (:then_0
      (if (== (Variables|Global|GetRoundNumber) 30)
        (CallFunction|InitialAllVariables)
        (Viewport|RemoveAllWidgets)
        (bind _returnvalue (UserInterface|CreateWidget "/Game/BluePrints/WBP_GameOver.WBP_GameOver_C"))
        (Variables|/Game/BluePrints/WBP_GameOver.WBP_GameOver_C|SetWinner _returnvalue "平局")
        (UserInterface|Viewport|AddtoViewport _returnvalue 0)))
    (:then_1
      (if (Math|Boolean|ORBoolean (>= (Variables|City|GetP1Tower) 50) (== (Variables|City|GetP2Tower) 0) (== (Variables|CardNumber|GetP2Cards) 0))
        (CallFunction|InitialAllVariables)
        (Viewport|RemoveAllWidgets)
        (bind _returnvalue_2 (UserInterface|CreateWidget "/Game/BluePrints/WBP_GameOver.WBP_GameOver_C"))
        (Variables|/Game/BluePrints/WBP_GameOver.WBP_GameOver_C|SetWinner _returnvalue_2 (Utilities|Text|FormatText "{Winner}获胜!!" (Variables|Default|GetPlayer1Name)))
        (UserInterface|Viewport|AddtoViewport _returnvalue_2 0)))
    (:then_2
      (if (Math|Boolean|ORBoolean (>= (Variables|City|GetP2Tower) 50) (== (Variables|City|GetP1Tower) 0) (== (Variables|CardNumber|GetP1Cards) 0))
        (CallFunction|InitialAllVariables)
        (Viewport|RemoveAllWidgets)
        (bind _returnvalue_3 (UserInterface|CreateWidget "/Game/BluePrints/WBP_GameOver.WBP_GameOver_C"))
        (Variables|/Game/BluePrints/WBP_GameOver.WBP_GameOver_C|SetWinner _returnvalue_3 (Utilities|Text|FormatText "{Winner}获胜!!" (Variables|Default|GetPlayer2Name)))
        (UserInterface|Viewport|AddtoViewport _returnvalue_3 0)))))

(fn InitialAllVariables
  (Utilities|FlowControl|Sequence
    (:then_0
      (Variables|Resource|SetP1Brick 10))
    (:then_1
      (Variables|Resource|SetP1Gem 10))
    (:then_2
      (Variables|Resource|SetP1Monster 10))
    (:then_3
      (Variables|Resource|SetP2Gem 10))
    (:then_4
      (Variables|Resource|SetP2Brick 10))
    (:then_5
      (Variables|Resource|SetP2Monster 10))
    (:then_6
      (Variables|Resource|SetP1BrickOutput 2))
    (:then_7
      (Variables|Resource|SetP1GemOutput 2))
    (:then_8
      (Variables|Resource|SetP1MonsterOutput 2))
    (:then_9
      (Variables|Resource|SetP2BrickOutput 2))
    (:then_10
      (Variables|Resource|SetP2GemOutput 2))
    (:then_11
      (Variables|Resource|SetP2MonsterOutput 2))
    (:then_12
      (Variables|City|SetP1Tower 25))
    (:then_13
      (Variables|City|SetP1Rampart 10))
    (:then_14
      (Variables|City|SetP2Rampart 10))
    (:then_15
      (Variables|City|SetP2Tower 25))
    (:then_16
      (Variables|Default|SetPlayer1Name "Player1"))
    (:then_17
      (Variables|Default|SetPlayer2Name "Player2"))
    (:then_18
      (Variables|Global|SetCurrentPlayer true))
    (:then_19
      (Variables|Global|SetRoundNumber 1))
    (:then_20
      (Variables|Global|Setpos 12))
    (:then_21
      (Variables|Global|SetCurrentRound 1))
    (:then_22
      (Variables|Default|SetIsTest false))
    (:then_23
      (Variables|CardNumber|SetP1Cards 6))
    (:then_24
      (Variables|CardNumber|SetP2Cards 6))))